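; Manager that auto-generates sphere illumination volumes around lights, providing boundary overlaps for the illumination detection system.
; GenerateOverlaps scans all actors for point or spot light components, then spawns, initializes, sizes and attaches a BP_IlluminationSphereVolume to each match.
; It tracks spawned volumes in GeneratedOverlaps, so separate events can destroy them, leaving hand-placed volumes intact, or toggle their bounds visibility.
; An older PointLight/SpotLight class-based version remains as unused nodes.
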(event `GenerateOverlaps`
  ;[1 1 1] Gets a reference to all point & spot light components, spawns, assigns & initializes Sphere Illumination Volumes to them for boundary overlap functionality
  (bind _outactors (`GameplayStatics.GetAllActorsOfClass` "/Script/Engine.Actor"))
  (for _array_element _outactors
    (if (or (`KismetSystemLibrary.IsValid` (`self.GetComponentByClass` _array_element "/Script/Engine.PointLightComponent")) (`KismetSystemLibrary.IsValid` (`self.GetComponentByClass` _array_element "/Script/Engine.SpotLightComponent")))
      (bind _returnvalue (`|SpawnActorFromClass` "/Game/IlluminationDetection/Blueprints/IlluminationVolumes/BP_IlluminationSphereVolume.BP_IlluminationSphereVolume_C" (`self.GetTransform` _array_element) "AlwaysSpawn" "OverrideRootScale" null null))
      (`KismetArrayLibrary.Array_Add` (`self.GeneratedOverlaps`) _returnvalue)
      (set `/Game/IlluminationDetection/Blueprints/IlluminationVolumes/BP_IlluminationVolumeMaster.LightActorRef` _array_element _returnvalue)
      (`/Game/IlluminationDetection/Blueprints/IlluminationVolumes/BP_IlluminationVolumeMaster.Initialize` _returnvalue)
      (`/Game/IlluminationDetection/Blueprints/IlluminationVolumes/BP_IlluminationSphereVolume.SetBoundRadius` _returnvalue)
      (`self.K2_AttachToActor` _returnvalue _array_element "None" "SnapToTarget" "SnapToTarget" "SnapToTarget" true))))

(event `RemoveGeneratedOverlaps`
  ;[1 1 1] Clears any illumination volumes spawned by this actor, doesn't remove manually placed volumes
  (for _array_element (`self.GeneratedOverlaps`)
    (`self.K2_DestroyActor` _array_element))
  (`KismetArrayLibrary.Array_Clear` (`self.GeneratedOverlaps`)))

(event `ShowOverlapBounds`
  ;[1 1 1] Toggle Bounds Visibility at Runtime
  (for _array_element (`self.GeneratedOverlaps`)
    (`/Game/IlluminationDetection/Blueprints/IlluminationVolumes/BP_IlluminationVolumeMaster.UpdateBoundsVisibility` _array_element false)))

(event `HideOverlapBounds`
  ;[1 1 1] Toggle Bounds Visibility at Runtime
  (for _array_element (`self.GeneratedOverlaps`)
    (`/Game/IlluminationDetection/Blueprints/IlluminationVolumes/BP_IlluminationVolumeMaster.UpdateBoundsVisibility` _array_element true)))

(fn `UserConstructionScript`)