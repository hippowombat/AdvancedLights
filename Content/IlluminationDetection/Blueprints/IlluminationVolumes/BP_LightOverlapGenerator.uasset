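; Generator actor that places sphere illumination volumes on the level's point and spot lights to provide boundary overlaps for illumination detection.
; GenerateOverlaps spawns a BP_IlluminationSphereVolume at each light's transform, assigns the light reference, then initializes it and sets its bound radius.
; Spawned volumes are tracked in GeneratedOverlaps, so RemoveGeneratedOverlaps destroys only those, leaving manually placed volumes intact.
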(event `GenerateOverlaps`
  ;[1 1 1] Gets a reference to all point & spot lights, spawns, assigns & initializes Sphere Illumination Volumes to them for boundary overlap functionality
  (bind _outactors (`GameplayStatics.GetAllActorsOfClass` "/Script/Engine.PointLight"))
  (for _array_element _outactors
    (bind _returnvalue (`|SpawnActorFromClass` "/Game/IlluminationDetection/Blueprints/IlluminationVolumes/BP_IlluminationSphereVolume.BP_IlluminationSphereVolume_C" (`self.GetTransform` _array_element) "AlwaysSpawn" "OverrideRootScale" null null))
    (`KismetArrayLibrary.Array_Add` (`self.GeneratedOverlaps`) _returnvalue)
    (set `/Game/IlluminationDetection/Blueprints/IlluminationVolumes/BP_IlluminationVolumeMaster.PointLightRef` _array_element _returnvalue)
    (`/Game/IlluminationDetection/Blueprints/IlluminationVolumes/BP_IlluminationVolumeMaster.Initialize` _returnvalue)
    (`/Game/IlluminationDetection/Blueprints/IlluminationVolumes/BP_IlluminationSphereVolume.SetBoundRadius` _returnvalue))
  (bind _outactors_2 (`GameplayStatics.GetAllActorsOfClass` "/Script/Engine.SpotLight"))
  (for _array_element_2 _outactors_2
    (bind _returnvalue_2 (`|SpawnActorFromClass` "/Game/IlluminationDetection/Blueprints/IlluminationVolumes/BP_IlluminationSphereVolume.BP_IlluminationSphereVolume_C" (`self.GetTransform` _array_element_2) "AlwaysSpawn" "OverrideRootScale" null null))
    (`KismetArrayLibrary.Array_Add` (`self.GeneratedOverlaps`) _returnvalue_2)
    (set `/Game/IlluminationDetection/Blueprints/IlluminationVolumes/BP_IlluminationVolumeMaster.SpotLightRef` _array_element_2 _returnvalue_2)
    (`/Game/IlluminationDetection/Blueprints/IlluminationVolumes/BP_IlluminationVolumeMaster.Initialize` _returnvalue_2)
    (`/Game/IlluminationDetection/Blueprints/IlluminationVolumes/BP_IlluminationSphereVolume.SetBoundRadius` _returnvalue_2)))

(event `RemoveGeneratedOverlaps`
  (bind _generatedoverlaps (`self.GeneratedOverlaps`))
  ;[1 1 1] Clears any illumination volumes spawned by this actor, doesn't remove manually placed volumes
  (for _array_element _generatedoverlaps
    (`self.K2_DestroyActor` _array_element))
  (`KismetArrayLibrary.Array_Clear` (`self.GeneratedOverlaps`))
  (`KismetSystemLibrary.PrintString` (`KismetStringLibrary.Conv_IntToString` (`KismetArrayLibrary.Array_Length` _generatedoverlaps))))

(fn `UserConstructionScript`)