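; Spherical illumination volume actor that makes itself known to illumination probes within its bounds for evaluation.
; On BeginPlay and begin overlap, it adds itself to the volume array of each BP_IlluminationProbe component on overlapping actors, removing itself on end overlap.
; Construction sizes the sphere from the parent's extent and applies debug visibility.
; A manual radius update serves the overlap generator, and an event toggles bounds visibility for debugging.
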(event `self.ReceiveBeginPlay`
  ;[1 1 1] Boundary overlaps give references to this actor instance to the overlapping probe for evaulation, self-removes on end overlap for clean operation throughout
  (`parent.ReceiveBeginPlay`)
  (for _array_element (`PrimitiveComponent.GetOverlappingActors` (`self.SphereBounds`) "/Script/Engine.Actor")
    (for _array_element_2 (`self.K2_GetComponentsByClass` _array_element "/Game/IlluminationDetection/Blueprints/IlluminationComponents/BP_IlluminationProbe.BP_IlluminationProbe_C")
      (`KismetArrayLibrary.Array_Add` (`/Game/IlluminationDetection/Blueprints/IlluminationComponents/BP_IlluminationProbe.ArrayMV` _array_element_2) self))))

(event `self.SphereBounds.OnComponentBeginOverlap`
  (params (OverlappedComponent :type "PrimitiveComponent Object Reference") (OtherActor :type "Actor Object Reference") (OtherComp :type "PrimitiveComponent Object Reference") (OtherBodyIndex :type Integer) (bFromSweep :type Boolean) (SweepResult :type "HitResult Structure (by ref)"))
  ;[1 1 1] Boundary overlaps give references to this actor instance to the overlapping probe for evaulation, self-removes on end overlap for clean operation throughout
  (for _array_element (`self.K2_GetComponentsByClass` OtherActor "/Game/IlluminationDetection/Blueprints/IlluminationComponents/BP_IlluminationProbe.BP_IlluminationProbe_C")
    (`KismetArrayLibrary.Array_Add` (`/Game/IlluminationDetection/Blueprints/IlluminationComponents/BP_IlluminationProbe.ArrayMV` _array_element) self)))

(event `self.SphereBounds.OnComponentEndOverlap`
  (params (OverlappedComponent :type "PrimitiveComponent Object Reference") (OtherActor :type "Actor Object Reference") (OtherComp :type "PrimitiveComponent Object Reference") (OtherBodyIndex :type Integer))
  ;[1 1 1] Boundary overlaps give references to this actor instance to the overlapping probe for evaulation, self-removes on end overlap for clean operation throughout
  (for _array_element (`self.K2_GetComponentsByClass` OtherActor "/Game/IlluminationDetection/Blueprints/IlluminationComponents/BP_IlluminationProbe.BP_IlluminationProbe_C")
    (`KismetArrayLibrary.Array_RemoveItem` (`/Game/IlluminationDetection/Blueprints/IlluminationComponents/BP_IlluminationProbe.ArrayMV` _array_element) self)))

(event `self.UpdateBoundsVisibility`
  (params (`HiddenInGame?` :type Boolean))
  ;[1 1 1] Update Boundary Visibility (for debugging)
  (`SceneComponent.SetHiddenInGame` (`self.SphereBounds`) `HiddenInGame?` false))

(fn `SetBoundRadius`
  ;[1 1 1] Manual function to update sphere radius, used in overlap generator
  (`SphereComponent.SetSphereRadius` (`self.SphereBounds`) (`self.VolumeSphereExtent`) true))

(fn `UserConstructionScript`
  (`parent.UserConstructionScript`)
  ;[1 1 1] Set sphere volume bounds & bounds visibility from parent extent variables
  (`SphereComponent.SetSphereRadius` (`self.SphereBounds`) (`self.VolumeSphereExtent`) true)
  (`SceneComponent.SetHiddenInGame` (`self.SphereBounds`) (not (`self.DebugBounds?`)) false))