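; Blueprint function library for the illumination detection system that combines an array of light probes into one overall illumination value.
; CheckOverallIllumination multiplies each probe's illumination by that probe's MaxOverallIllumination weight and adds it to a running total.
; The total is clamped between zero and one at every step, so the result is a capped weighted sum rather than an average.
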(fn `CheckOverallIllumination`
  (params (IlluminationProbes :type "Array of /Game/IlluminationDetection/Blueprints/IlluminationComponents/BP_IlluminationProbe Object Reference"))
  (returns (OverallIllumination :type "Float (double-precision)"))
  (locals (TempIlluminationVal :type "Float (double-precision)"))
  ;[1 1 1] Compares illumination value of all light probes in an array & provides an overall illumination value across the board
  (set `local.TempIlluminationVal` 0.0)
  (for _array_element IlluminationProbes
    (set `local.TempIlluminationVal` (`KismetMathLibrary.FClamp` (+ (`local.TempIlluminationVal`) (* (`/Game/IlluminationDetection/Blueprints/IlluminationComponents/BP_IlluminationProbe.MaxOverallIllumination` _array_element) (`/Game/IlluminationDetection/Blueprints/IlluminationComponents/BP_IlluminationProbe.ProbeIllumination` _array_element))))))
  (return (`local.TempIlluminationVal`)))