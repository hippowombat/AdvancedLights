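; BP_IlluminationCubeVolume is a box volume that registers itself with BP_SmartLightProbe components on actors inside it.
; On BeginPlay it adds itself to the ArrayMV list of each probe on actors already overlapping BoxBounds.
; Begin and end overlap events on BoxBounds then add or remove it from those lists as actors enter and leave.
; The construction script sizes BoxBounds from VolumeBoxExtent.
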(event `self.ReceiveBeginPlay`
  (`parent.ReceiveBeginPlay`)
  (for _array_element (`PrimitiveComponent.GetOverlappingActors` (`self.BoxBounds`) "/Script/Engine.Actor")
    (for _array_element_2 (`self.K2_GetComponentsByClass` _array_element "/Game/Blueprints/BP_SmartLightProbe.BP_SmartLightProbe_C")
      (`KismetArrayLibrary.Array_Add` (`/Game/Blueprints/BP_SmartLightProbe.ArrayMV` _array_element_2) self))))

(event `self.BoxBounds.OnComponentBeginOverlap`
  (params (OverlappedComponent :type "PrimitiveComponent Object Reference") (OtherActor :type "Actor Object Reference") (OtherComp :type "PrimitiveComponent Object Reference") (OtherBodyIndex :type Integer) (bFromSweep :type Boolean) (SweepResult :type "HitResult Structure (by ref)"))
  (for _array_element (`self.K2_GetComponentsByClass` OtherActor "/Game/Blueprints/BP_SmartLightProbe.BP_SmartLightProbe_C")
    (`KismetArrayLibrary.Array_Add` (`/Game/Blueprints/BP_SmartLightProbe.ArrayMV` _array_element) self)))

(event `self.BoxBounds.OnComponentEndOverlap`
  (params (OverlappedComponent :type "PrimitiveComponent Object Reference") (OtherActor :type "Actor Object Reference") (OtherComp :type "PrimitiveComponent Object Reference") (OtherBodyIndex :type Integer))
  (for _array_element (`self.K2_GetComponentsByClass` OtherActor "/Game/Blueprints/BP_SmartLightProbe.BP_SmartLightProbe_C")
    (`KismetArrayLibrary.Array_RemoveItem` (`/Game/Blueprints/BP_SmartLightProbe.ArrayMV` _array_element) self)))

(fn `UserConstructionScript`
  (`parent.UserConstructionScript`)
  (`BoxComponent.SetBoxExtent` (`self.BoxBounds`) (`self.VolumeBoxExtent`) true))