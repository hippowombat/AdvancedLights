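; Master Blueprint for a manually placed illumination volume, defined by box and sphere extents and a local source location.
; Its construction script sets AttenuationDistance to the largest of the box's three axis extents and the sphere extent.
; A helper converts SourceLocation into world space through the actor transform; the event graph has no active logic.
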(fn `GetAttenuationDistanceFromAllExtentAxes`
  (returns (Return :type Boolean))
  (locals (TempMaxDist :type "Float (double-precision)") (Extents :type "Array of Float (double-precision)") (CurrentHighestInstance :type Integer :default -1))
  (bind (_volumeboxextent_x _volumeboxextent_y _volumeboxextent_z) (`KismetMathLibrary.BreakVector` (`self.VolumeBoxExtent`)))
  (set `local.TempMaxDist` 0.0)
  (set `local.CurrentHighestInstance` -1)
  (bind _output_get (set `local.Extents` (`|MakeArray` _volumeboxextent_x _volumeboxextent_y _volumeboxextent_z (`self.VolumeSphereExtent`))))
  (for (_array_element _array_index) _output_get
    (if (> _array_element (`local.TempMaxDist`))
      (set `local.TempMaxDist` _array_element)
      (set `local.CurrentHighestInstance` _array_index)))
  (if (>= (`local.CurrentHighestInstance`) 0)
    (set `self.AttenuationDistance` (`|GetArrayItem` (`local.Extents`) (`local.CurrentHighestInstance`)))
    (return true)
    (else
      (return false))))

(fn `GetWorldspaceSourceLocation`
  (returns (ReturnValue :type "Vector Structure"))
  (return (`KismetMathLibrary.TransformLocation` (`self.GetTransform`) (`self.SourceLocation`))))

(fn `UserConstructionScript`
  (`self.GetAttenuationDistanceFromAllExtentAxes`))