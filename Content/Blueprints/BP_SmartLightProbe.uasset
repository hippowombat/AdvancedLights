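; Light probe component that measures how lit its world location is, every tick.
; It line-traces to point, spot (cone-tested), ArrayMV and optional directional lights, and optionally counts sky lights untraced.
; Visible lights add their BP_LightIlluminationProperties MaxIllumination, scaled by distance falloff for all but directional and sky lights.
; It stores visible count, in-light flag and clamped illumination, then calls UpdateLightRangeStatus; debug trace drawing is on.
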(event `self.ReceiveTick`
  (params (DeltaSeconds :type "Float (single-precision)"))
  (`self.DetectLightVis`))

(fn `DetectLightVis`
  (locals (TempVisCount :type Integer) (TempIlluminationVal :type "Float (double-precision)"))
  (bind _returnvalue (`self.K2_GetComponentLocation`))
  (set `local.TempVisCount` 0)
  (set `local.TempIlluminationVal` 0.0)
  ;[1 1 1] Point Light Probe Check
  (for _array_element (`self.ArrayPL`)
    (bind _outhit (`KismetSystemLibrary.LineTraceSingle` :`Start` (`self.K2_GetComponentLocation`) :`End` (`Actor.K2_GetActorLocation` _array_element) :`TraceChannel` "TraceTypeQuery1" :`DrawDebugType` (`self.DebugTraceLine`)))
    (bind (_bblockinghit _binitialoverlap _time _distance _location _impactpoint _normal _impactnormal _physmat _hitactor _hitcomponent _hitbonename _hititem _faceindex _tracestart _traceend) (`GameplayStatics.BreakHitResult` _outhit))
    (if (not _bblockinghit)
      (`/Engine/EditorBlueprintResources/StandardMacros.IncrementInt` (`local.TempVisCount`)
        (:`  `
          (set `local.TempIlluminationVal` (+ (`local.TempIlluminationVal`) (* (`KismetMathLibrary.FClamp` (- 1.0 (/ (`KismetMathLibrary.VSize` (- _tracestart _traceend)) (`LocalLightComponent.AttenuationRadius` (`PointLight.PointLightComponent` _array_element))))) (`/Game/Blueprints/BP_LightIlluminationProperties.MaxIllumination` (`/Game/Blueprints/BP_SmartPointLight.BP_LightIlluminationProperties` _array_element)))))))))
  (for _array_element_2 (`self.ArrayMV`)
    (bind _outhit_2 (`KismetSystemLibrary.LineTraceSingle` :`Start` (`self.K2_GetComponentLocation`) :`End` (`/Game/Blueprints/BP_ManualIlluminationVolumeMaster.GetWorldspaceSourceLocation` _array_element_2) :`TraceChannel` "TraceTypeQuery1" :`DrawDebugType` (`self.DebugTraceLine`) :`TraceColor` (struct :`R` 1.0 :`G` 0.25 :`B` 0.75 :`A` 1.0)))
    (bind (_bblockinghit_2 _binitialoverlap_2 _time_2 _distance_2 _location_2 _impactpoint_2 _normal_2 _impactnormal_2 _physmat_2 _hitactor_2 _hitcomponent_2 _hitbonename_2 _hititem_2 _faceindex_2 _tracestart_2 _traceend_2) (`GameplayStatics.BreakHitResult` _outhit_2))
    (if (not _bblockinghit_2)
      (`/Engine/EditorBlueprintResources/StandardMacros.IncrementInt` (`local.TempVisCount`)
        (:`  `
          (set `local.TempIlluminationVal` (+ (`local.TempIlluminationVal`) (* (`KismetMathLibrary.FClamp` (- 1.0 (/ (`KismetMathLibrary.VSize` (- _tracestart_2 _traceend_2)) (`/Game/Blueprints/BP_ManualIlluminationVolumeMaster.AttenuationDistance` _array_element_2)))) (`/Game/Blueprints/BP_LightIlluminationProperties.MaxIllumination` (`/Game/Blueprints/BP_ManualIlluminationVolumeMaster.BP_LightIlluminationProperties` _array_element_2)))))))))
  (for _array_element_3 (`self.ArraySL`)
    (if (>= (`KismetMathLibrary.Dot_VectorVector` (`Actor.GetActorForwardVector` _array_element_3) (`KismetMathLibrary.Conv_RotatorToVector` (`KismetMathLibrary.FindLookAtRotation` (`Actor.K2_GetActorLocation` _array_element_3) (`self.K2_GetComponentLocation`)))) (- 1.0 (/ (`SpotLightComponent.OuterConeAngle` (`SpotLight.SpotLightComponent` _array_element_3)) 180.0)))
      (bind _outhit_3 (`KismetSystemLibrary.LineTraceSingle` :`Start` (`self.K2_GetComponentLocation`) :`End` (`Actor.K2_GetActorLocation` _array_element_3) :`TraceChannel` "TraceTypeQuery1" :`DrawDebugType` (`self.DebugTraceLine`) :`TraceColor` (struct :`R` 1.0 :`G` 1.0 :`B` 0.2 :`A` 1.0)))
      (bind (_bblockinghit_3 _binitialoverlap_3 _time_3 _distance_3 _location_3 _impactpoint_3 _normal_3 _impactnormal_3 _physmat_3 _hitactor_3 _hitcomponent_3 _hitbonename_3 _hititem_3 _faceindex_3 _tracestart_3 _traceend_3) (`GameplayStatics.BreakHitResult` _outhit_3))
      (if (not _bblockinghit_3)
        (`/Engine/EditorBlueprintResources/StandardMacros.IncrementInt` (`local.TempVisCount`)
          (:`  `
            (set `local.TempIlluminationVal` (+ (`local.TempIlluminationVal`) (* (`KismetMathLibrary.FClamp` (- 1.0 (/ (`KismetMathLibrary.VSize` (- _tracestart_3 _traceend_3)) (`LocalLightComponent.AttenuationRadius` (`SpotLight.SpotLightComponent` _array_element_3))))) (`/Game/Blueprints/BP_LightIlluminationProperties.MaxIllumination` (`/Game/Blueprints/BP_SmartSpotlight.BP_LightIlluminationProperties` _array_element_3))))))))))
  (if (`self.CheckDirectionalLights?`)
    (bind _outactors (`GameplayStatics.GetAllActorsOfClass` "/Script/Engine.DirectionalLight"))
    (for _array_element_4 _outactors
      (bind _outhit_4 (`KismetSystemLibrary.LineTraceSingle` :`Start` _returnvalue :`End` (+ _returnvalue (* (`Actor.GetActorForwardVector` _array_element_4) (* (`self.DirectionalLightTraceDistance`) -1.0))) :`TraceChannel` "TraceTypeQuery1" :`DrawDebugType` (`self.DebugTraceLine`) :`TraceColor` (struct :`R` 0.2 :`G` 1.0 :`B` 1.0 :`A` 1.0) :`DrawTime` 0.0))
      (if (not (`GameplayStatics.BreakHitResult` _outhit_4))
        (`/Engine/EditorBlueprintResources/StandardMacros.IncrementInt` (`local.TempVisCount`)
          (:`  `
            (bind _returnvalue_2 (`Actor.K2_GetComponentsByClass` _array_element_4 "/Game/Blueprints/BP_LightIlluminationProperties.BP_LightIlluminationProperties_C"))
            (if (> (`KismetArrayLibrary.Array_Length` _returnvalue_2) 0)
              (set `local.TempIlluminationVal` (+ (`local.TempIlluminationVal`) (`/Game/Blueprints/BP_LightIlluminationProperties.MaxIllumination` (`|GetArrayItem` _returnvalue_2))))))))))
  (if (`self.CheckSkyLights?`)
    (bind _outactors_2 (`GameplayStatics.GetAllActorsOfClass` "/Script/Engine.SkyLight"))
    (for _array_element_5 _outactors_2
      (`/Engine/EditorBlueprintResources/StandardMacros.IncrementInt` (`local.TempVisCount`)
        (:`  `
          (bind _returnvalue_3 (`Actor.K2_GetComponentsByClass` _array_element_5 "/Game/Blueprints/BP_LightIlluminationProperties.BP_LightIlluminationProperties_C"))
          (if (> (`KismetArrayLibrary.Array_Length` _returnvalue_3) 0)
            (set `local.TempIlluminationVal` (+ (`local.TempIlluminationVal`) (`/Game/Blueprints/BP_LightIlluminationProperties.MaxIllumination` (`|GetArrayItem` _returnvalue_3)))))))))
  (bind _output_get (set `self.LightVisCount` (`local.TempVisCount`)))
  (set `self.IsWithinRangeOfLight` (> _output_get 0))
  (bind _output_get_2 (set `self.ProbeIllumination` (`KismetMathLibrary.FClamp` (`local.TempIlluminationVal`))))
  (`self.UpdateLightRangeStatus`)
  (return))