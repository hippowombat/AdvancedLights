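; BP_SmartSpotlight is a spotlight that registers itself with BP_SmartLightProbe components through their ArraySL lists.
; The construction script sizes the ConeBounds sphere to the light's attenuation radius and tints the pointer arrow to the light color.
; BeginPlay registers with probes on actors already inside the sphere.
; Overlap begin and end add or remove it, but look up probes on the spotlight itself, not the overlapping actor.
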(event `self.ReceiveBeginPlay`
  (for _array_element (`PrimitiveComponent.GetOverlappingActors` (`self.ConeBounds`) "/Script/Engine.Actor")
    (for _array_element_2 (`self.K2_GetComponentsByClass` _array_element "/Game/Blueprints/BP_SmartLightProbe.BP_SmartLightProbe_C")
      (`KismetArrayLibrary.Array_Add` (`/Game/Blueprints/BP_SmartLightProbe.ArraySL` _array_element_2) self))))

(event `self.ReceiveTick`
  (params (DeltaSeconds :type "Float (single-precision)")))

(event `self.ConeBounds.OnComponentBeginOverlap`
  (params (OverlappedComponent :type "PrimitiveComponent Object Reference") (OtherActor :type "Actor Object Reference") (OtherComp :type "PrimitiveComponent Object Reference") (OtherBodyIndex :type Integer) (bFromSweep :type Boolean) (SweepResult :type "HitResult Structure (by ref)"))
  (for _array_element (`self.K2_GetComponentsByClass` "/Game/Blueprints/BP_SmartLightProbe.BP_SmartLightProbe_C")
    (`KismetArrayLibrary.Array_Add` (`/Game/Blueprints/BP_SmartLightProbe.ArraySL` _array_element) self)))

(event `self.ConeBounds.OnComponentEndOverlap`
  (params (OverlappedComponent :type "PrimitiveComponent Object Reference") (OtherActor :type "Actor Object Reference") (OtherComp :type "PrimitiveComponent Object Reference") (OtherBodyIndex :type Integer))
  (for _array_element (`self.K2_GetComponentsByClass` "/Game/Blueprints/BP_SmartLightProbe.BP_SmartLightProbe_C")
    (`KismetArrayLibrary.Array_RemoveItem` (`/Game/Blueprints/BP_SmartLightProbe.ArraySL` _array_element) self)))

(fn `UserConstructionScript`
  (`SphereComponent.SetSphereRadius` (`self.ConeBounds`) (`LocalLightComponent.AttenuationRadius` (`self.SpotLightComponent`)) true)
  (`ArrowComponent.SetArrowColor` (`self.SpotlightPointer`) (`LightComponentBase.GetLightColor` (`self.SpotLightComponent`))))