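; BP_TestProbe is a test actor that shows whether any of its BP_SmartLightProbe components is within range of a light.
; The construction script gathers those probes and binds their range-status updates to UpdateLightStatus.
; Each update rechecks all probes and colors VisArrow red if any is lit, otherwise green.
; BeginPlay sets TestTimeline's play rate, but the timeline that would lerp Test between two locations is never started.
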(event `self.ReceiveBeginPlay`
  (`TimelineComponent.SetPlayRate` (`self.TestTimeline`) (`self.TestTimelineSpeed`)))

(event `EventStoreLightProbes`
  (bind _output_get (set `self.LightProbes` (`self.K2_GetComponentsByClass` "/Game/Blueprints/BP_SmartLightProbe.BP_SmartLightProbe_C")))
  (for _array_element _output_get
    (add `/Game/Blueprints/BP_SmartLightProbe.UpdateLightRangeStatus` _array_element (delegate `UpdateLightStatus`))))

(event `UpdateLightStatus`
  (bind _anyprobesinlight_ (`self.CheckForLight`))
  (`ArrowComponent.SetArrowColor` (`self.VisArrow`) (`KismetMathLibrary.SelectColor` (struct :`G` 1.0 :`A` 1.0) (struct :`R` 1.0 :`A` 1.0) (not _anyprobesinlight_))))

(fn `CheckForLight`
  (returns (`AnyProbesInLight?` :type Boolean))
  (locals (`Seen?` :type Boolean))
  (set `local.Seen?` false)
  (for _array_element (`self.LightProbes`)
    (if (`/Game/Blueprints/BP_SmartLightProbe.IsWithinRangeOfLight` _array_element)
      (set `local.Seen?` true)
      (break)))
  (return (`local.Seen?`)))

(fn `UserConstructionScript`
  (`self.EventStoreLightProbes`))