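; Stealth example spawner that manages a capped number of cop pawns (BP_Pawn with IsCop set) responding to calls at a chase location.
; CallCops destroys cops far from the player, redirects nearby ones with a new AI state and move speed, then spawns more.
; Spawning retries random offsets around the call location until a sphere trace above the point is clear, then places the whole batch there.
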(event `self.ReceiveBeginPlay`
  (bind _outactors (`GameplayStatics.GetAllActorsOfClass` "/Game/GameplayExamples/Stealth/Blueprints/BP_StealthCharacter.BP_StealthCharacter_C"))
  (set `self.PlayerReference` (`|GetArrayItem` _outactors)))

(event `CallCops`
  (params (ChaseLocation :type "Vector Structure"))
  (bind (_returnexistingcopsoutofrange _returnexistingcopsinrange) (`self.DetectExistingCops`))
  (set `self.CurrentCopCount` (- (`self.CurrentCopCount`) (`KismetArrayLibrary.Array_Length` _returnexistingcopsoutofrange)))
  (for _array_element _returnexistingcopsoutofrange
    (`self.K2_DestroyActor` _array_element))
  (for _array_element_2 _returnexistingcopsinrange
    (`/Engine/EditorBlueprintResources/StandardMacros.IsValid` _array_element_2
      (:`Is Valid`
        (set `/Game/GameplayExamples/Stealth/Blueprints/BP_Pawn.ChaseLocation` ChaseLocation _array_element_2)
        (bind _aicontroller (`/Game/GameplayExamples/Stealth/Blueprints/BP_Pawn.AIController` _array_element_2))
        (`/Engine/EditorBlueprintResources/StandardMacros.IsValid` _aicontroller
          (:`Is Valid`
            (bind _output_get (set `/Game/GameplayExamples/Stealth/Blueprints/BP_Pawn_Controller.AI_State` "NewEnumerator2" _aicontroller))
            (`/Game/GameplayExamples/Stealth/Blueprints/BP_Pawn.UpdateMoveSpeed` _array_element_2 _output_get))))))
  (`self.SpawnCops` ChaseLocation))

(event `SpawnCops`
  (params (CallLocation :type "Vector Structure"))
  (bind (_sucess_ _loc) (`self.GetRandomSpawnLoc` CallLocation :!label _label))
  (if _sucess_
    (if (> (- (- (`self.MaxCopsAllowed`) (`self.CurrentCopCount`)) 1) 0)
      (for _ (range (- (`self.MaxCopsAllowed`) (`self.CurrentCopCount`)))
        (bind _returnvalue (`|SpawnActorFromClass` "/Game/GameplayExamples/Stealth/Blueprints/BP_Pawn.BP_Pawn_C" (`KismetMathLibrary.MakeTransform` _loc) "AdjustIfPossibleButAlwaysSpawn" "OverrideRootScale" null null))
        (set `/Game/GameplayExamples/Stealth/Blueprints/BP_Pawn.IsCop` true _returnvalue)
        (set `/Game/GameplayExamples/Stealth/Blueprints/BP_Pawn.ChaseLocation` CallLocation _returnvalue)
        (`/Engine/EditorBlueprintResources/StandardMacros.IncrementInt` (`self.CurrentCopCount`))))
    (else
      (goto _label))))

(event `self.ReceiveTick`
  (params (DeltaSeconds :type "Float (single-precision)")))

(fn `DetectExistingCops`
  (returns (ReturnExistingCopsOutOfRange :type "Array of /Game/GameplayExamples/Stealth/Blueprints/BP_Pawn Object Reference") (ReturnExistingCopsInRange :type "Array of /Game/GameplayExamples/Stealth/Blueprints/BP_Pawn Object Reference"))
  (locals (ExistingCopsInRange :type "Array of /Game/GameplayExamples/Stealth/Blueprints/BP_Pawn Object Reference") (ExistingCopsOutOfRange :type "Array of /Game/GameplayExamples/Stealth/Blueprints/BP_Pawn Object Reference"))
  (bind _outactors (`GameplayStatics.GetAllActorsOfClass` "/Game/GameplayExamples/Stealth/Blueprints/BP_Pawn.BP_Pawn_C"))
  (for _array_element _outactors
    (if (`/Game/GameplayExamples/Stealth/Blueprints/BP_Pawn.IsCop` _array_element)
      (if (< (`KismetMathLibrary.VSize` (- (`self.K2_GetActorLocation` _array_element) (`self.K2_GetActorLocation` (`self.PlayerReference`)))) 5000.0)
        (`KismetArrayLibrary.Array_Add` (`local.ExistingCopsInRange`) _array_element)
        (else
          (`KismetArrayLibrary.Array_Add` (`local.ExistingCopsOutOfRange`) _array_element)))))
  (return (`local.ExistingCopsOutOfRange`) (`local.ExistingCopsInRange`)))

(fn `GetRandomSpawnLoc`
  (params (A :type "Vector Structure"))
  (returns (`Sucess?` :type Boolean) (Loc :type "Vector Structure"))
  (locals (TempLoc :type "Vector Structure"))
  (bind _returnvalue (`KismetMathLibrary.SelectFloat` (`KismetMathLibrary.RandomFloatInRange` -5000.0 -2500.0) (`KismetMathLibrary.RandomFloatInRange` 5000.0 2500.0) (`KismetMathLibrary.RandomBool`)))
  (bind _returnvalue_2 (+ (`local.TempLoc`) (0.0 0.0 1000.0)))
  (set `local.TempLoc` (+ A (`KismetMathLibrary.MakeVector` _returnvalue _returnvalue)))
  (bind (_outhit _returnvalue_3) (`KismetSystemLibrary.SphereTraceSingle` _returnvalue_2 _returnvalue_2 200.0 "TraceTypeQuery1" true))
  (if _returnvalue_3
    (return false (0.0 0.0 0.0))
    (else
      (return true (`local.TempLoc`)))))

(fn `UserConstructionScript`)