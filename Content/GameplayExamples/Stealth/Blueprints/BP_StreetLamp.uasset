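; Street lamp prop for the stealth gameplay example, assembled parametrically in the Construction Script with no runtime logic.
; BaseScale and MidScale size the two post sections, which are stacked by height on the assumption of 100-unit, center-pivot meshes.
; LampHead sits on top of the stack, and a child actor is added at a rotated, forward and raised offset from that point.
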(fn `UserConstructionScript`
  (bind _basescale (`self.BaseScale`))
  (bind _midscale (`self.MidScale`))
  (bind _z (.z _basescale))
  (bind _z_2 (.z _midscale))
  (bind _returnvalue (* _z 100.0))
  (bind _returnvalue_2 (+ _returnvalue (* _z_2 100.0)))
  (`SceneComponent.SetRelativeScale3D` (`self.Base`) _basescale)
  (`SceneComponent.K2_SetRelativeLocation` (`self.Base`) (`KismetMathLibrary.MakeVector` 0.0 0.0 (* (/ _z 2.0) 100.0)) false false)
  (`SceneComponent.SetRelativeScale3D` (`self.Mid`) _midscale)
  (`SceneComponent.K2_SetRelativeLocation` (`self.Mid`) (`KismetMathLibrary.MakeVector` 0.0 0.0 (+ (* (/ _z_2 2.0) 100.0) _returnvalue)) false false)
  (`SceneComponent.K2_SetRelativeLocation` (`self.LampHead`) (`KismetMathLibrary.MakeVector` 0.0 0.0 _returnvalue_2) false false)
  (`AddComponent|NODE_AddChildActorComponent-0` :`RelativeTransform` (`KismetMathLibrary.MakeTransform` (`KismetMathLibrary.MakeVector` 68.519997 0.0 (+ _returnvalue_2 50.0)) (struct :`Pitch` -90.0))))