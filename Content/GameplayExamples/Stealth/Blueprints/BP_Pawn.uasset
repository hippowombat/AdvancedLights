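; Stealth-example NPC pawn that acts as a patrolling civilian or, with IsCop set, a chasing cop.
; Each tick, a trace with distance, facing and illumination checks spots a player who is BeingWeird, driving head look-at and a camera-facing signal widget.
; Interact runs odds-based pickpocketing, with failures forcing a bump.
; Gated bumps make the pawn jump and, if repeated or the player is weird, call police through BP_CopSpawner.
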(event `self.ReceiveBeginPlay`
  (`KismetSystemLibrary.Delay` 0.1)
  (`self.Initialize`)
  (bind _outactors (`GameplayStatics.GetAllActorsOfClass` "/Game/GameplayExamples/Stealth/Blueprints/BP_StealthCharacter.BP_StealthCharacter_C"))
  (set `self.PlayerRef` (`|GetArrayItem` _outactors))
  (bind _outactors_2 (`GameplayStatics.GetAllActorsOfClass` "/Script/Engine.Character"))
  (set `self.IgnoreActors` _outactors_2)
  (bind _aswb_signal (cast `/Game/GameplayExamples/Stealth/Blueprints/UI/WB_Signal` (`WidgetComponent.GetUserWidgetObject` (`self.Sig`))))
  (set `self.SigWidgetRef` _aswb_signal))

(event `Initialize`
  (bind _asbp_pawn_controller (cast `/Game/GameplayExamples/Stealth/Blueprints/BP_Pawn_Controller` (`AIBlueprintHelperLibrary.GetAIController` self)))
  (if (`self.IsCop`)
    (set `CharacterMovementComponent.MaxWalkSpeed` 480.0 (`self.CharacterMovement`))
    (bind _output_get (set `self.AIController` _asbp_pawn_controller))
    (set `/Game/GameplayExamples/Stealth/Blueprints/BP_Pawn_Controller.ControlledPawn` self _output_get)
    (set `/Game/GameplayExamples/Stealth/Blueprints/BP_Pawn_Controller.AI_State` "NewEnumerator2" (`self.AIController`))
    (set `self.CashInPocket` (`KismetMathLibrary.RandomIntegerInRange` 12 30))
    (`PrimitiveComponent.SetMaterial` (`self.Mesh`) 0 "/Game/GameplayExamples/Stealth/Materials/Instances/MI_Cop.MI_Cop")
    (`SceneComponent.SetVisibility` (`self.Hat`) (`self.IsCop`) false)
    (`SceneComponent.SetVisibility` (`self.Sunglasses`) (`self.IsCop`) false)
    (else
      (bind _patrolpath (`self.PatrolPath`)
        (:`then`
          (set `/Game/GameplayExamples/Stealth/Blueprints/BP_Pawn_Controller.PatrolPoints` (`/Game/GameplayExamples/Stealth/Blueprints/BP_PatrolPath.Locations` _patrolpath) _asbp_pawn_controller)
          (set `self.AIController` _asbp_pawn_controller))
        (:`else`)))))

(event `EventBump`
  ;[1 1 1] Bump/Agitate Pawns
  (`|ExecutionSequence`
    (:`then_0`
      (`/Engine/EditorBlueprintResources/StandardMacros.Gate` false :!label _label
        (:`Exit`
          (`self.Jump`)
          (`/Engine/EditorBlueprintResources/StandardMacros.IncrementInt` (`self.TimesBumped`)
            (:`  `
              (`|ExecutionSequence`
                (:`then_0`
                  (`KismetSystemLibrary.Delay` 0.5)
                  (goto _label :!via `Open`))
                (:`then_1`
                  (if (or (`/Game/GameplayExamples/Stealth/Blueprints/BP_StealthCharacter.BeingWeird` (`self.PlayerRef`)) (> (`self.TimesBumped`) 3))
                    (`self.CallCops`)))))))))
    (:`then_1`
      (goto _label :!via `Close`))))

(event `/Game/GameplayExamples/Stealth/Blueprints/BP_InteractionInterface.Interact`
  (params (Instigator :type "Actor Object Reference") (SuccessOdds :type "Float (single-precision)"))
  ;[1 1 1] Odds-driven pickpocketing
  (bind _asbp_stealth_character (cast `/Game/GameplayExamples/Stealth/Blueprints/BP_StealthCharacter` Instigator))
  (if (and (> (* SuccessOdds 0.01) (`KismetMathLibrary.RandomFloatInRange` 0.0 1.0)) (> (`self.CashInPocket`) 0))
    (`/Game/GameplayExamples/Stealth/Blueprints/BP_InteractionInterface.PickPocket` _asbp_stealth_character (`self.CashInPocket`))
    (set `self.CashInPocket` 0)
    (else
      (`self.ForceBump`))))

(event `ForceBump`
  ;[1 1 1] Bump/Agitate Pawns
  (`|ExecutionSequence`
    (:`then_0`
      (goto _label :!via `Open`))
    (:`then_1`
      (goto _label))))

(event `CallCops`
  ;[1 1 1] Bump/Agitate Pawns
  (bind _outactors (`GameplayStatics.GetAllActorsOfClass` "/Game/GameplayExamples/Stealth/Blueprints/BP_CopSpawner.BP_CopSpawner_C"))
  (`/Game/GameplayExamples/Stealth/Blueprints/BP_CopSpawner.CallCops` (`|GetArrayItem` _outactors) (`self.K2_GetActorLocation`))
  (set `/Game/GameplayExamples/Stealth/Blueprints/BP_Pawn_Controller.AI_State` "NewEnumerator3" (`self.AIController`)))

(event `self.ReceiveTick`
  (params (DeltaSeconds :type "Float (single-precision)"))
  (bind _playerref (`self.PlayerRef`))
  ;[1 1 1] Face signal UI element to player
  (`SceneComponent.K2_SetWorldRotation` (`self.Sig`) (`KismetMathLibrary.FindLookAtRotation` (`SceneComponent.K2_GetComponentLocation` (`self.Sig`)) (`PlayerCameraManager.GetCameraLocation` (`GameplayStatics.GetPlayerCameraManager` 0))) false false)
  ;[1 1 1] LookAtCode
  (bind _playerref_2 (`self.PlayerRef`)
    (:`then`
      (bind _outhit (`KismetSystemLibrary.LineTraceSingle` (`SceneComponent.GetSocketLocation` (`self.Mesh`) "NogginSocket") (`SceneComponent.GetSocketLocation` (`Character.Mesh` _playerref_2) "NogginSocket") "TraceTypeQuery2" false (`self.IgnoreActors`)))
      (bind _returnvalue (`KismetMathLibrary.FindLookAtRotation` (`SceneComponent.GetSocketLocation` (`self.Mesh`) "NogginSocket") (`SceneComponent.GetSocketLocation` (`Character.Mesh` _playerref_2) "NogginSocket")))
      (bind _returnvalue_2 (and (not (`GameplayStatics.BreakHitResult` _outhit)) (< (`KismetMathLibrary.VSize` (- (`.TraceStart` (`GameplayStatics.BreakHitResult` _outhit)) (`.TraceEnd` (`GameplayStatics.BreakHitResult` _outhit)))) (`self.VisionDistance`)) (> (`KismetMathLibrary.Dot_VectorVector` (`self.GetActorForwardVector`) (`KismetMathLibrary.Conv_RotatorToVector` _returnvalue)) 0.2) (`/Game/GameplayExamples/Stealth/Blueprints/BP_StealthCharacter.BeingWeird` _playerref) (>= (`/Game/GameplayExamples/Stealth/Blueprints/BP_StealthCharacter.CharacterIllumination` _playerref) 0.19)))
      (bind _output_get (set `self.SeesAWeirdDude` _returnvalue_2))
      (if (`|EnumEquality` (`/Game/GameplayExamples/Stealth/Blueprints/BP_Pawn_Controller.AI_State` (`self.AIController`)) "NewEnumerator3")
        (set `self.Signal` "NewEnumerator2")
        (elif (`self.IsCop`)
          (set `self.Signal` (select `bool` _output_get :`false` "NewEnumerator0" :`true` "NewEnumerator2" :!type "/Game/GameplayExamples/Stealth/Blueprints/EN_SignalStates Enum"))
          (else
            (set `self.Signal` (select `bool` _output_get :`false` "NewEnumerator0" :`true` "NewEnumerator1" :!type "/Game/GameplayExamples/Stealth/Blueprints/EN_SignalStates Enum")))))
      (`/Game/GameplayExamples/Stealth/Blueprints/UI/WB_Signal.UpdateWidget` (`self.SigWidgetRef`) (`self.Signal`))
      (set `self.LookAtRot` (`KismetMathLibrary.RInterpTo` (`self.LookAtRot`) (`KismetMathLibrary.SelectRotator` (`KismetMathLibrary.MakeRotator` (* (.pitch _returnvalue) -1.0) (- (.yaw _returnvalue) (.yaw (`self.K2_GetActorRotation`))) (.roll _returnvalue)) (struct) _returnvalue_2) (`GameplayStatics.GetWorldDeltaSeconds`) 5.0)))
    (:`else`
      (set `self.LookAtRot` (struct)))))

(fn `RandomizeClothing`
  (params (Mat :type "MaterialInstanceDynamic Object Reference") (`Randomize?` :type Boolean))
  (if `Randomize?`
    (`MaterialInstanceDynamic.SetVectorParameterValue` Mat "RedColor" (`self.ShirtColor`))
    (`MaterialInstanceDynamic.SetVectorParameterValue` Mat "BlueColor" (`self.PantsColor`))))

(fn `UpdateMoveSpeed`
  (params (AIState :type "/Game/GameplayExamples/Stealth/Blueprints/EN_AIStates Enum" :default "NewEnumerator0"))
  (set `CharacterMovementComponent.MaxWalkSpeed` (select `/Game/GameplayExamples/Stealth/Blueprints/EN_AIStates` AIState :`NewEnumerator0` 450.0 :`NewEnumerator1` 125.0 :`NewEnumerator2` 450.0 :!type "Float (single-precision)") (`self.CharacterMovement`)))

(fn `UserConstructionScript`
  (set `self.RandomInt` (`KismetMathLibrary.RandomIntegerInRange` 0 9))
  (set `self.ShirtColor` (select `int` (`self.RandomInt`) :`0` (struct :`R` 0.958333 :`G` 0.958333 :`B` 0.958333 :`A` 1.0) :`1` (struct :`R` 0.302083 :`G` 0.302083 :`B` 0.302083 :`A` 1.0) :`2` (struct :`R` 0.005208 :`G` 0.005208 :`B` 0.005208 :`A` 1.0) :`3` (struct :`R` 0.447917 :`G` 0.216266 :`B` 0.252066 :`A` 1.0) :`4` (struct :`R` 0.265341 :`G` 0.16517 :`B` 0.338542 :`A` 1.0) :`5` (struct :`R` 0.198172 :`G` 0.40625 :`B` 0.120605 :`A` 1.0) :`6` (struct :`R` 0.765625 :`G` 0.649091 :`B` 0.040622 :`A` 1.0) :`7` (struct :`R` 0.347333 :`G` 0.364583 :`B` 0.23341 :`A` 1.0) :`8` (struct :`R` 0.229063 :`G` 0.070095 :`B` 0.354167 :`A` 1.0) :`9` (struct :`G` 0.385417 :`B` 0.137081 :`A` 1.0) :!type "LinearColor Structure"))
  (set `self.PantsColor` (select `int` (`self.RandomInt`) :`0` (struct :`R` 0.019608 :`G` 0.07451 :`B` 0.168627 :`A` 1.0) :`1` (struct :`R` 0.019608 :`G` 0.07451 :`B` 0.168627 :`A` 1.0) :`2` (struct :`R` 0.019608 :`G` 0.07451 :`B` 0.168627 :`A` 1.0) :`3` (struct :`R` 0.019608 :`G` 0.07451 :`B` 0.168627 :`A` 1.0) :`4` (struct :`R` 0.019608 :`G` 0.07451 :`B` 0.168627 :`A` 1.0) :`5` (struct :`R` 0.019608 :`G` 0.07451 :`B` 0.168627 :`A` 1.0) :`6` (struct :`R` 0.019608 :`G` 0.07451 :`B` 0.168627 :`A` 1.0) :`7` (struct :`R` 0.011765 :`G` 0.011765 :`B` 0.011765 :`A` 1.0) :`8` (struct :`R` 0.011765 :`G` 0.011765 :`B` 0.011765 :`A` 1.0) :`9` (struct :`R` 0.011765 :`G` 0.011765 :`B` 0.011765 :`A` 1.0) :!type "LinearColor Structure"))
  (bind _returnvalue (`KismetMaterialLibrary.CreateDynamicMaterialInstance` "/Game/GameplayExamples/Stealth/Materials/Instances/MI_PawnCharacter.MI_PawnCharacter"))
  (`PrimitiveComponent.SetMaterial` (`self.Mesh`) 1 _returnvalue)
  (`self.RandomizeClothing` _returnvalue)
  (set `self.CashInPocket` (`KismetMathLibrary.RandomIntegerInRange` 2 12))
  (`SceneComponent.SetVisibility` (`self.Hat`) (`self.IsCop`) false)
  (`SceneComponent.SetVisibility` (`self.Sunglasses`) (`self.IsCop`) false)
  (set `self.LookAtRot` (`KismetMathLibrary.MakeRotator` (* (.pitch (`KismetMathLibrary.FindLookAtRotation` (`SceneComponent.GetSocketLocation` (`self.Mesh`) "NogginSocket") (`KismetMathLibrary.TransformLocation` (`self.GetTransform`) (`self.TempLookAtLocation`)))) -1.0) (- (.yaw (`KismetMathLibrary.FindLookAtRotation` (`SceneComponent.GetSocketLocation` (`self.Mesh`) "NogginSocket") (`KismetMathLibrary.TransformLocation` (`self.GetTransform`) (`self.TempLookAtLocation`)))) (.yaw (`self.K2_GetActorRotation`))) (.roll (`KismetMathLibrary.FindLookAtRotation` (`SceneComponent.GetSocketLocation` (`self.Mesh`) "NogginSocket") (`KismetMathLibrary.TransformLocation` (`self.GetTransform`) (`self.TempLookAtLocation`)))))))