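; Player character for the stealth gameplay example that tracks how brightly lit it is.
; Input events drive crouch toggling, control-rotation-relative movement and yaw-only turning.
; Each tick it copies the illumination value from its head illumination probe into CharacterIllumination and prints it on screen for debugging.
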(event `InputAction|Crouch`
  (params (Key :type "Key Structure"))
  ;[1 1 1] BaseMovement
  (:`Pressed`
    (if (`self.bIsCrouched`)
      (`self.UnCrouch`)
      (else
        (`self.Crouch`)))))

(event `InputAxis|MoveForward`
  (params (AxisValue :type "Float (single-precision)"))
  ;[1 1 1] BaseMovement
  (`self.AddMovementInput` (`KismetMathLibrary.GetForwardVector` (`self.GetControlRotation`)) AxisValue))

(event `InputAxis|MoveRight`
  (params (AxisValue :type "Float (single-precision)"))
  ;[1 1 1] BaseMovement
  (`self.AddMovementInput` (`KismetMathLibrary.GetRightVector` (`self.GetControlRotation`)) AxisValue))

(event `InputAxis|TurnRate`
  (params (AxisValue :type "Float (single-precision)"))
  ;[1 1 1] BaseMovement
  (`self.AddControllerYawInput` AxisValue))

(event `InputAxis|Turn`
  (params (AxisValue :type "Float (single-precision)"))
  ;[1 1 1] BaseMovement
  (`self.AddControllerYawInput` AxisValue))

(event `self.ReceiveTick`
  (params (DeltaSeconds :type "Float (single-precision)"))
  (bind _output_get (set `self.CharacterIllumination` (`/Game/IlluminationDetection/Blueprints/IlluminationComponents/BP_IlluminationProbe.ProbeIllumination` (`self.BP_IlluminationProbeHead`))))
  (`KismetSystemLibrary.PrintString` (`KismetStringLibrary.Conv_DoubleToString` _output_get) true true (struct :`G` 0.66 :`B` 1.0 :`A` 1.0) 0.0))

(fn `UserConstructionScript`)