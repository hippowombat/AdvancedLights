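; AI controller for BP_Pawn in the stealth gameplay example, driving it along a patrol route.
; On BeginPlay it starts a looping timer at AIFrequency in place of Tick, caches the pawn and sets its move speed from AIState.
; Each timer call switches on AIState; only Patrol has logic, moving to the current patrol point and advancing the index on success, resetting once it exceeds the array length.
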(event `self.ReceiveBeginPlay`
  (`KismetSystemLibrary.K2_SetTimerDelegate` (delegate `AI_Function`) (`self.AI_Frequency`) true)
  (bind _asbp_pawn (cast `/Game/GameplayExamples/Stealth/Blueprints/BP_Pawn` (`self.K2_GetPawn`)))
  (bind _output_get (set `self.ControlledPawn` _asbp_pawn))
  (`/Game/GameplayExamples/Stealth/Blueprints/BP_Pawn.UpdateMoveSpeed` _output_get (`self.AI_State`)))

(event `AI_Function`
  (switch `/Game/GameplayExamples/Stealth/Blueprints/EN_AIStates` (`self.AI_State`)
    (:`NewEnumerator1`
      (`|AIMoveTo` (`self.K2_GetPawn`) (`|GetArrayItem` (`self.PatrolPoints`) (`self.CurrentPatrolPoint`)) null 25.0
        (:`OnSuccess`
          (bind _output_get (set `self.CurrentPatrolPoint` (+ (`self.CurrentPatrolPoint`) 1)))
          (if (> _output_get (`KismetArrayLibrary.Array_Length` (`self.PatrolPoints`)))
            (set `self.CurrentPatrolPoint` 0)))))))

(fn `UserConstructionScript`)