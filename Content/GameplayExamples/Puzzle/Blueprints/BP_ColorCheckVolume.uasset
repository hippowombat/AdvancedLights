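; Puzzle volume that opens a linked gate when the player's physics ball is inside it with a matching light color.
; Each Tick it tests the ball's distance against the sphere radius instead of using overlap events, then fires the gate once on a match.
; A match requires each RGB channel to be within a tolerance of the target color.
; The construction script sizes the sphere and glow cylinder and tints the cylinder with the target color.
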(event `self.ReceiveBeginPlay`
  (bind _outactors (`GameplayStatics.GetAllActorsOfClass` "/Game/GameplayExamples/Puzzle/Blueprints/PhysicsBallBP.PhysicsBallBP_C"))
  (set `self.PlayerRef` (`|GetArrayItem` _outactors)))

(event `OpenDoor`
  (bind _gatetoopen (`self.GateToOpen`)
    (:`then`
      (`/Game/GameplayExamples/Puzzle/Blueprints/BP_Gate.OpenGate` _gatetoopen))
    (:`else`)))

(event `self.ReceiveTick`
  (params (DeltaSeconds :type "Float (single-precision)"))
  (if (< (`KismetMathLibrary.VSize` (- (`self.K2_GetActorLocation`) (`SceneComponent.K2_GetComponentLocation` (`/Game/GameplayExamples/Puzzle/Blueprints/PhysicsBallBP.Ball` (`self.PlayerRef`))))) (`SphereComponent.SphereRadius` (`self.Sphere`)))
    (if (`self.DoesColorMatch?`)
      (`/Engine/EditorBlueprintResources/StandardMacros.DoOnce` false
        (:`Completed`
          (`self.OpenDoor`))))))

(fn `DoesColorMatch?`
  (returns (ReturnValue :type Boolean))
  (bind (_r _g _b) (`KismetMathLibrary.BreakColor` (`self.CompareColor`)))
  (bind (_r_2 _g_2 _b_2) (`KismetMathLibrary.BreakColor` (`/Game/GameplayExamples/Puzzle/Blueprints/PhysicsBallBP.BallLightColor` (`self.PlayerRef`))))
  (return (>= (+ (`KismetMathLibrary.SelectInt` 1 0 (`KismetMathLibrary.NearlyEqual_FloatFloat` _r_2 _r (`self.ColorMatchRange`))) (`KismetMathLibrary.SelectInt` 1 0 (`KismetMathLibrary.NearlyEqual_FloatFloat` _g_2 _g (`self.ColorMatchRange`))) (`KismetMathLibrary.SelectInt` 1 0 (`KismetMathLibrary.NearlyEqual_FloatFloat` _b_2 _b (`self.ColorMatchRange`)))) 3)))

(fn `UserConstructionScript`
  (bind _returnvalue (/ (`self.VolumeRadius`) 50.0))
  (`SphereComponent.SetSphereRadius` (`self.Sphere`) (`self.VolumeRadius`) true)
  (`SceneComponent.SetRelativeScale3D` (`self.Cylinder`) (`KismetMathLibrary.MakeVector` _returnvalue _returnvalue (`self.CylinderHeight`)))
  (`SceneComponent.K2_SetRelativeLocation` (`self.Cylinder`) (`KismetMathLibrary.MakeVector` 0.0 0.0 (+ (* (`self.CylinderHeight`) 50.0) -5.0)) false false)
  (bind _returnvalue_2 (`PrimitiveComponent.CreateDynamicMaterialInstance` (`self.Cylinder`) 0 "/Game/GameplayExamples/Puzzle/Materials/MI_CylinderGlow.MI_CylinderGlow" "None"))
  (`MaterialInstanceDynamic.SetVectorParameterValue` _returnvalue_2 "Color" (`self.CompareColor`)))