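; Watering can actor that the first-person character can pick up, tilt and drop, with a fake water surface inside.
; Pickup attaches it to the character's GrabSphere, Rotate applies clamped roll, and Drop restarts handle physics and resets rotation.
; A vector curve maps fill value to water scale and height, applied at construction.
; Tick updates water position and, while held, counter-rotates it by half the can's roll.
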(event `self.ReceiveTick`
  (params (DeltaSeconds :type "Float (single-precision)"))
  (bind (_returnvalue_x _returnvalue_y _returnvalue_z) (`KismetMathLibrary.BreakVector` (`CurveVector.GetVectorValue` (`self.WaterValuesCurve`) (`self.WaterCanFillValue`))))
  (bind _relativerotation_roll (`KismetMathLibrary.BreakRotator` (`SceneComponent.RelativeRotation` (`self.WaterCan`))))
  (bind _returnvalue (/ (- 0.0 _relativerotation_roll) 2.0))
  (`SceneComponent.K2_SetRelativeLocationAndRotation` (`self.SM_Water`) (`KismetMathLibrary.MakeVector` 0.0 (`KismetMathLibrary.Lerp` 0.0 (`self.WaterMaxTiltOffset`) (`KismetMathLibrary.Abs` (/ (`KismetMathLibrary.FClamp` _returnvalue -25.0 0.0) -25.0))) _returnvalue_z) (`KismetMathLibrary.MakeRotator` (`KismetMathLibrary.SelectFloat` _returnvalue 0.0 (`self.IsPickedup`))) false false))

(event `EventUpdateWaterValues`
  (bind (_returnvalue_x _returnvalue_y _returnvalue_z) (`KismetMathLibrary.BreakVector` (`CurveVector.GetVectorValue` (`self.WaterValuesCurve`) (`self.WaterCanFillValue`))))
  (`SceneComponent.SetRelativeScale3D` (`self.SM_Water`) (* (1.0 1.0 1.0) (`KismetMathLibrary.FClamp` _returnvalue_x 0.01 500.0)))
  (`SceneComponent.K2_SetRelativeLocation` (`self.SM_Water`) (`KismetMathLibrary.MakeVector` 0.0 0.0 _returnvalue_z) false false))

(event `/Game/GameplayExamples/Plant/Blueprints/IF_Pickup.Pickup`
  (params (AttachActor :type "Actor Object Reference"))
  (bind _asfirst_person_character (cast `/Game/FirstPersonBP/Blueprints/FirstPersonCharacter` AttachActor))
  (`self.K2_AttachToComponent` (`/Game/FirstPersonBP/Blueprints/FirstPersonCharacter.GrabSphere` _asfirst_person_character) "None" "SnapToTarget" "KeepWorld" "KeepWorld" true)
  (`KismetSystemLibrary.PrintString` "Hello")
  (set `self.IsPickedup` true))

(event `/Game/GameplayExamples/Plant/Blueprints/IF_Pickup.Drop`
  (bind _watercanhandle (`self.WaterCanHandle`))
  (`self.K2_DetachFromActor` "KeepWorld" "KeepWorld" "KeepWorld")
  (`PrimitiveComponent.SetSimulatePhysics` _watercanhandle false)
  (`PrimitiveComponent.SetSimulatePhysics` _watercanhandle true)
  (set `self.IsPickedup` false)
  (`self.K2_SetActorRotation` (struct) true))

(event `/Game/GameplayExamples/Plant/Blueprints/IF_Pickup.Rotate`
  (params (RotVal :type "Float (single-precision)"))
  (bind _relativerotation_roll (`KismetMathLibrary.BreakRotator` (`SceneComponent.RelativeRotation` (`self.WaterCan`))))
  (`SceneComponent.K2_SetRelativeRotation` (`self.WaterCan`) (`KismetMathLibrary.MakeRotator` (`KismetMathLibrary.FClamp` (+ RotVal _relativerotation_roll) -25.0 0.0)) false false))

(fn `UserConstructionScript`
  (`self.EventUpdateWaterValues`))